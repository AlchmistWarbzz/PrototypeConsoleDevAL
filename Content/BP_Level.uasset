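; Level actor that runs a staged level: clear four enemy triggers, fight a boss, then return to MainMenu.
; Overlap boxes destroy paired cubes, count enemies, or switch the camera between this actor and the player.
; Tick polls the counters, revealing solid portal cubes after four enemies and after twenty boss hits, which also destroy the boss.
; Hitting a portal teleports the character, swaps camera view and toggles each area's lights.
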(event `self.ReceiveBeginPlay`
  (`PrimitiveComponent.SetCollisionEnabled` (`self.Cube9`) "NoCollision")
  (`PrimitiveComponent.SetCollisionEnabled` (`self.Cube10`) "NoCollision"))

(event `self.Cube9.OnComponentHit`
  (params (HitComponent :type "PrimitiveComponent Object Reference") (OtherActor :type "Actor Object Reference") (OtherComp :type "PrimitiveComponent Object Reference") (NormalImpulse :type "Vector Structure") (Hit :type "HitResult Structure (by ref)"))
  (bind (_teleport1_location _teleport1_rotation) (`KismetMathLibrary.BreakTransform` (`self.Teleport1`)))
  (`PlayerController.SetViewTargetWithBlend` (`GameplayStatics.GetPlayerController` 0) self 0.0 "VTBlend_Linear" 0.0 false)
  (`SceneComponent.SetVisibility` (`self.PointLight5`) true false)
  (`SceneComponent.SetVisibility` (`self.PointLight4`) true false)
  (`SceneComponent.SetVisibility` (`self.BossFight`) true false)
  (`SceneComponent.SetVisibility` (`self.Cube8`) true false)
  (`SceneComponent.SetVisibility` (`self.PointLight1`) false false)
  (`SceneComponent.SetVisibility` (`self.PointLight2`) false false)
  (`SceneComponent.SetVisibility` (`self.PointLight`) false false)
  (`SceneComponent.SetVisibility` (`self.PaperFlipbook`) false false)
  (`SceneComponent.SetVisibility` (`self.PointLight3`) false false)
  (bind _asbp_third_person_character (cast `/Game/ThirdPerson/Blueprints/BP_ThirdPersonCharacter` OtherActor))
  (`self.K2_SetActorLocationAndRotation` _asbp_third_person_character (`KismetMathLibrary.TransformLocation` (`self.GetTransform`) _teleport1_location) _teleport1_rotation false true))

(event `self.Box1.OnComponentBeginOverlap`
  (params (OverlappedComponent :type "PrimitiveComponent Object Reference") (OtherActor :type "Actor Object Reference") (OtherComp :type "PrimitiveComponent Object Reference") (OtherBodyIndex :type Integer) (bFromSweep :type Boolean) (SweepResult :type "HitResult Structure (by ref)"))
  (`ActorComponent.K2_DestroyComponent` (`self.Cube3`))
  (`ActorComponent.K2_DestroyComponent` (`self.Cube1`)))

(event `self.Box6.OnComponentBeginOverlap`
  (params (OverlappedComponent :type "PrimitiveComponent Object Reference") (OtherActor :type "Actor Object Reference") (OtherComp :type "PrimitiveComponent Object Reference") (OtherBodyIndex :type Integer) (bFromSweep :type Boolean) (SweepResult :type "HitResult Structure (by ref)"))
  (set `self.Enemies` (+ (`self.Enemies`) 1.0))
  (`ActorComponent.K2_DestroyComponent` (`self.Box6`))
  (`ActorComponent.K2_DestroyComponent` (`self.Cube7`)))

(event `self.Box5.OnComponentBeginOverlap`
  (params (OverlappedComponent :type "PrimitiveComponent Object Reference") (OtherActor :type "Actor Object Reference") (OtherComp :type "PrimitiveComponent Object Reference") (OtherBodyIndex :type Integer) (bFromSweep :type Boolean) (SweepResult :type "HitResult Structure (by ref)"))
  (set `self.Enemies` (+ (`self.Enemies`) 1.0))
  (`ActorComponent.K2_DestroyComponent` (`self.Box5`))
  (`ActorComponent.K2_DestroyComponent` (`self.Cube6`)))

(event `self.Box2.OnComponentBeginOverlap`
  (params (OverlappedComponent :type "PrimitiveComponent Object Reference") (OtherActor :type "Actor Object Reference") (OtherComp :type "PrimitiveComponent Object Reference") (OtherBodyIndex :type Integer) (bFromSweep :type Boolean) (SweepResult :type "HitResult Structure (by ref)"))
  (`ActorComponent.K2_DestroyComponent` (`self.Cube2`))
  (`ActorComponent.K2_DestroyComponent` (`self.Cube`)))

(event `self.Box3.OnComponentBeginOverlap`
  (params (OverlappedComponent :type "PrimitiveComponent Object Reference") (OtherActor :type "Actor Object Reference") (OtherComp :type "PrimitiveComponent Object Reference") (OtherBodyIndex :type Integer) (bFromSweep :type Boolean) (SweepResult :type "HitResult Structure (by ref)"))
  (set `self.Enemies` (+ (`self.Enemies`) 1.0))
  (`ActorComponent.K2_DestroyComponent` (`self.Box3`))
  (`ActorComponent.K2_DestroyComponent` (`self.Cube4`)))

(event `self.Box7.OnComponentBeginOverlap`
  (params (OverlappedComponent :type "PrimitiveComponent Object Reference") (OtherActor :type "Actor Object Reference") (OtherComp :type "PrimitiveComponent Object Reference") (OtherBodyIndex :type Integer) (bFromSweep :type Boolean) (SweepResult :type "HitResult Structure (by ref)"))
  (bind _asbp_third_person_character (cast `/Game/ThirdPerson/Blueprints/BP_ThirdPersonCharacter` OtherActor))
  (`PlayerController.SetViewTargetWithBlend` (`GameplayStatics.GetPlayerController` 0) _asbp_third_person_character 0.0 "VTBlend_Linear" 0.0 false))

(event `self.Box4.OnComponentBeginOverlap`
  (params (OverlappedComponent :type "PrimitiveComponent Object Reference") (OtherActor :type "Actor Object Reference") (OtherComp :type "PrimitiveComponent Object Reference") (OtherBodyIndex :type Integer) (bFromSweep :type Boolean) (SweepResult :type "HitResult Structure (by ref)"))
  (set `self.Enemies` (+ (`self.Enemies`) 1.0))
  (`ActorComponent.K2_DestroyComponent` (`self.Box4`))
  (`ActorComponent.K2_DestroyComponent` (`self.Cube5`)))

(event `self.ReceiveTick`
  (params (DeltaSeconds :type "Float (single-precision)"))
  (bind _cube10 (`self.Cube10`))
  (if (>= (`self.Enemies`) 4.0)
    (`SceneComponent.SetVisibility` (`self.Cube9`) true false)
    (`PrimitiveComponent.SetCollisionEnabled` (`self.Cube9`) "QueryAndPhysics")
    (if (>= (`self.Boss`) 20.0)
      (`ActorComponent.K2_DestroyComponent` (`self.BossFight`))
      (`SceneComponent.SetVisibility` _cube10 true false)
      (`SceneComponent.SetVisibility` (`self.PointLight6`) true false)
      (`PrimitiveComponent.SetCollisionEnabled` _cube10 "QueryAndPhysics"))))

(event `self.Box8.OnComponentBeginOverlap`
  (params (OverlappedComponent :type "PrimitiveComponent Object Reference") (OtherActor :type "Actor Object Reference") (OtherComp :type "PrimitiveComponent Object Reference") (OtherBodyIndex :type Integer) (bFromSweep :type Boolean) (SweepResult :type "HitResult Structure (by ref)"))
  (`PlayerController.SetViewTargetWithBlend` (`GameplayStatics.GetPlayerController` 0) self 0.0 "VTBlend_Linear" 0.0 false))

(event `self.Box9.OnComponentBeginOverlap`
  (params (OverlappedComponent :type "PrimitiveComponent Object Reference") (OtherActor :type "Actor Object Reference") (OtherComp :type "PrimitiveComponent Object Reference") (OtherBodyIndex :type Integer) (bFromSweep :type Boolean) (SweepResult :type "HitResult Structure (by ref)"))
  (bind _asbp_third_person_character (cast `/Game/ThirdPerson/Blueprints/BP_ThirdPersonCharacter` OtherActor))
  (`PlayerController.SetViewTargetWithBlend` (`GameplayStatics.GetPlayerController` 0) _asbp_third_person_character 0.0 "VTBlend_Linear" 0.0 false))

(event `self.Cube10.OnComponentHit`
  (params (HitComponent :type "PrimitiveComponent Object Reference") (OtherActor :type "Actor Object Reference") (OtherComp :type "PrimitiveComponent Object Reference") (NormalImpulse :type "Vector Structure") (Hit :type "HitResult Structure (by ref)"))
  (bind (_teleport2_location _teleport2_rotation) (`KismetMathLibrary.BreakTransform` (`self.Teleport2`)))
  (bind _asbp_third_person_character (cast `/Game/ThirdPerson/Blueprints/BP_ThirdPersonCharacter` OtherActor))
  (`PlayerController.SetViewTargetWithBlend` (`GameplayStatics.GetPlayerController` 0) _asbp_third_person_character 0.0 "VTBlend_Linear" 0.0 false)
  (`SceneComponent.SetVisibility` (`self.PointLight7`) true false)
  (`SceneComponent.SetVisibility` (`self.PointLight8`) true false)
  (`SceneComponent.SetVisibility` (`self.PointLight9`) true false)
  (`SceneComponent.SetVisibility` (`self.PointLight11`) true false)
  (`SceneComponent.SetVisibility` (`self.PointLight10`) true false)
  (`SceneComponent.SetVisibility` (`self.PointLight5`) false false)
  (`SceneComponent.SetVisibility` (`self.PointLight4`) false false)
  (bind _asbp_third_person_character_2 (cast `/Game/ThirdPerson/Blueprints/BP_ThirdPersonCharacter` OtherActor))
  (`self.K2_SetActorLocationAndRotation` _asbp_third_person_character_2 (`KismetMathLibrary.TransformLocation` (`self.GetTransform`) _teleport2_location) _teleport2_rotation false true))

(event `self.BossFight.OnComponentHit`
  (params (HitComponent :type "PrimitiveComponent Object Reference") (OtherActor :type "Actor Object Reference") (OtherComp :type "PrimitiveComponent Object Reference") (NormalImpulse :type "Vector Structure") (Hit :type "HitResult Structure (by ref)"))
  (set `self.Boss` (+ (`self.Boss`) 1.0)))

(event `self.Box10.OnComponentBeginOverlap`
  (params (OverlappedComponent :type "PrimitiveComponent Object Reference") (OtherActor :type "Actor Object Reference") (OtherComp :type "PrimitiveComponent Object Reference") (OtherBodyIndex :type Integer) (bFromSweep :type Boolean) (SweepResult :type "HitResult Structure (by ref)"))
  (`ActorComponent.K2_DestroyComponent` (`self.Cube8`))
  (`ActorComponent.K2_DestroyComponent` (`self.Box10`)))

(event `self.Box.OnComponentBeginOverlap`
  (params (OverlappedComponent :type "PrimitiveComponent Object Reference") (OtherActor :type "Actor Object Reference") (OtherComp :type "PrimitiveComponent Object Reference") (OtherBodyIndex :type Integer) (bFromSweep :type Boolean) (SweepResult :type "HitResult Structure (by ref)"))
  (`GameplayStatics.OpenLevel` "MainMenu"))

(fn `UserConstructionScript`)
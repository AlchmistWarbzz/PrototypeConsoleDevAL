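; BP_Elevator is an elevator actor that instantly teleports the third-person player character between a second floor and a boss floor.
; Two overlap boxes act as triggers: Box sends the character to TeleportSecondFloor and Box1 to TeleportBossFloor.
; Destination locations are converted from the elevator's local space, while rotations are applied directly.
; The second-floor trip sets the player camera view to the character, while the boss-floor trip sets it to the elevator actor.
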(event `self.Box.OnComponentBeginOverlap`
  (params (OverlappedComponent :type "PrimitiveComponent Object Reference") (OtherActor :type "Actor Object Reference") (OtherComp :type "PrimitiveComponent Object Reference") (OtherBodyIndex :type Integer) (bFromSweep :type Boolean) (SweepResult :type "HitResult Structure (by ref)"))
  (bind (_teleport_second_floor_location _teleport_second_floor_rotation) (`KismetMathLibrary.BreakTransform` (`self.Teleport Second Floor`)))
  (bind _asbp_third_person_character (cast `/Game/ThirdPerson/Blueprints/BP_ThirdPersonCharacter` OtherActor))
  (`self.K2_SetActorLocationAndRotation` _asbp_third_person_character (`KismetMathLibrary.TransformLocation` (`self.GetTransform`) _teleport_second_floor_location) _teleport_second_floor_rotation false true)
  (`PlayerController.SetViewTargetWithBlend` (`GameplayStatics.GetPlayerController` 0) _asbp_third_person_character 0.0 "VTBlend_Linear" 0.0 false))

(event `self.Box1.OnComponentBeginOverlap`
  (params (OverlappedComponent :type "PrimitiveComponent Object Reference") (OtherActor :type "Actor Object Reference") (OtherComp :type "PrimitiveComponent Object Reference") (OtherBodyIndex :type Integer) (bFromSweep :type Boolean) (SweepResult :type "HitResult Structure (by ref)"))
  (bind (_teleport_boss_floor_location _teleport_boss_floor_rotation) (`KismetMathLibrary.BreakTransform` (`self.Teleport Boss Floor`)))
  (bind _asbp_third_person_character (cast `/Game/ThirdPerson/Blueprints/BP_ThirdPersonCharacter` OtherActor))
  (`self.K2_SetActorLocationAndRotation` _asbp_third_person_character (`KismetMathLibrary.TransformLocation` (`self.GetTransform`) _teleport_boss_floor_location) _teleport_boss_floor_rotation false true)
  (`PlayerController.SetViewTargetWithBlend` (`GameplayStatics.GetPlayerController` 0) self 0.0 "VTBlend_Linear" 0.0 false))

(fn `UserConstructionScript`)
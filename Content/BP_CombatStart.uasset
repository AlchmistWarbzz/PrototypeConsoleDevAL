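; BP_CombatStart is a trigger actor that closes off a combat area and takes over the player's camera.
; Collision on five cube components is disabled at BeginPlay.
; Any overlap with Box1 makes the cubes visible and solid, then switches player 0's view target to this actor.
; The overlapping actor is not filtered, and nothing here reverses the lockdown or the camera switch.
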(event `self.ReceiveBeginPlay`
  (`PrimitiveComponent.SetCollisionEnabled` (`self.Cube`) "NoCollision")
  (`PrimitiveComponent.SetCollisionEnabled` (`self.Cube2`) "NoCollision")
  (`PrimitiveComponent.SetCollisionEnabled` (`self.Cube3`) "NoCollision")
  (`PrimitiveComponent.SetCollisionEnabled` (`self.Cube4`) "NoCollision")
  (`PrimitiveComponent.SetCollisionEnabled` (`self.Cube1`) "NoCollision"))

(event `self.Box1.OnComponentBeginOverlap`
  (params (OverlappedComponent :type "PrimitiveComponent Object Reference") (OtherActor :type "Actor Object Reference") (OtherComp :type "PrimitiveComponent Object Reference") (OtherBodyIndex :type Integer) (bFromSweep :type Boolean) (SweepResult :type "HitResult Structure (by ref)"))
  (bind _cube (`self.Cube`))
  (`SceneComponent.SetVisibility` _cube true false)
  (`SceneComponent.SetVisibility` (`self.Cube2`) true false)
  (`SceneComponent.SetVisibility` (`self.Cube3`) true false)
  (`SceneComponent.SetVisibility` (`self.Cube4`) true false)
  (`SceneComponent.SetVisibility` (`self.Cube1`) true false)
  (`PrimitiveComponent.SetCollisionEnabled` _cube "QueryAndPhysics")
  (`PrimitiveComponent.SetCollisionEnabled` (`self.Cube2`) "QueryAndPhysics")
  (`PrimitiveComponent.SetCollisionEnabled` (`self.Cube3`) "QueryAndPhysics")
  (`PrimitiveComponent.SetCollisionEnabled` (`self.Cube4`) "QueryAndPhysics")
  (`PrimitiveComponent.SetCollisionEnabled` (`self.Cube1`) "QueryAndPhysics")
  (`PlayerController.SetViewTargetWithBlend` (`GameplayStatics.GetPlayerController` 0) self 0.0 "VTBlend_Linear" 0.0 false))

(fn `UserConstructionScript`)
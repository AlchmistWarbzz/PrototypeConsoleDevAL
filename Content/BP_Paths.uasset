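; BP_Paths is an actor with two trigger boxes that teleport the third-person player character when overlapped.
; Box sends the character to the Teleport transform and Box1 to Teleport2, ignoring all other actors.
; Each target location is converted from actor-local to world space, while its rotation is applied as stored, without that conversion.
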(event `self.Box.OnComponentBeginOverlap`
  (params (OverlappedComponent :type "PrimitiveComponent Object Reference") (OtherActor :type "Actor Object Reference") (OtherComp :type "PrimitiveComponent Object Reference") (OtherBodyIndex :type Integer) (bFromSweep :type Boolean) (SweepResult :type "HitResult Structure (by ref)"))
  (bind (_teleport_location _teleport_rotation) (`KismetMathLibrary.BreakTransform` (`self.Teleport`)))
  (bind _asbp_third_person_character (cast `/Game/ThirdPerson/Blueprints/BP_ThirdPersonCharacter` OtherActor))
  (`self.K2_SetActorLocationAndRotation` _asbp_third_person_character (`KismetMathLibrary.TransformLocation` (`self.GetTransform`) _teleport_location) _teleport_rotation false true))

(event `self.Box1.OnComponentBeginOverlap`
  (params (OverlappedComponent :type "PrimitiveComponent Object Reference") (OtherActor :type "Actor Object Reference") (OtherComp :type "PrimitiveComponent Object Reference") (OtherBodyIndex :type Integer) (bFromSweep :type Boolean) (SweepResult :type "HitResult Structure (by ref)"))
  (bind (_teleport2_location _teleport2_rotation) (`KismetMathLibrary.BreakTransform` (`self.Teleport2`)))
  (bind _asbp_third_person_character (cast `/Game/ThirdPerson/Blueprints/BP_ThirdPersonCharacter` OtherActor))
  (`self.K2_SetActorLocationAndRotation` _asbp_third_person_character (`KismetMathLibrary.TransformLocation` (`self.GetTransform`) _teleport2_location) _teleport2_rotation false true))

(fn `UserConstructionScript`)